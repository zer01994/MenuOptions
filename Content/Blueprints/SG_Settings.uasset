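; SaveGame object that stores player settings: language, graphics and display command strings, master volume, mouse sensitivity and mouse invert.
; A setting-type enum selects the variable in both accessors, with separate string, float and bool channels for the value.
; LoadSettings returns the value held in memory without reading from disk.
; SaveSettings writes by reference through the Select, then saves the object itself to the "Settings" slot on every call.
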(fn `LoadSettings`
  (params (Type :type "/Game/Blueprints/Enum_Settings Enum" :default "NewEnumerator0"))
  (returns (StringType :type String) (FloatType :type "Float (double-precision)") (BoolType :type Boolean))
  (return (select `/Game/Blueprints/Enum_Settings` Type :`NewEnumerator0` (`self.LanguageCommand`) :`NewEnumerator1` (`self.GraphicCommand`) :`NewEnumerator2` (`self.PPCommand`) :`NewEnumerator3` (`self.AACommand`) :`NewEnumerator4` (`self.ShadowCommand`) :`NewEnumerator5` (`self.TQCommand`) :`NewEnumerator6` (`self.EQCommand`) :`NewEnumerator7` (`self.ResolutionCommand`) :`NewEnumerator8` (`self.ScreenCommand`) :`NewEnumerator9` (`self.MBCommand`) :`NewEnumerator10` (`self.VSyncCommand`) :`NewEnumerator11` (`self.ShadingCommand`)) (select `/Game/Blueprints/Enum_Settings` Type :`NewEnumerator12` (`self.MasterSound`) :`NewEnumerator13` (`self.Sensivity`)) (select `/Game/Blueprints/Enum_Settings` Type :`NewEnumerator14` (`self.MouseInvert`))))

(fn `SaveSettings`
  (params (Type :type "/Game/Blueprints/Enum_Settings Enum" :default "NewEnumerator0") (StringType :type String) (FloatType :type "Float (double-precision)") (BoolType :type Boolean))
  (switch `/Game/Blueprints/Enum_Settings` Type
    (:`NewEnumerator0`
      (`|VariableSetRef` (select `/Game/Blueprints/Enum_Settings` Type :`NewEnumerator0` (`self.LanguageCommand`) :`NewEnumerator1` (`self.GraphicCommand`) :`NewEnumerator2` (`self.PPCommand`) :`NewEnumerator3` (`self.AACommand`) :`NewEnumerator4` (`self.ShadowCommand`) :`NewEnumerator5` (`self.TQCommand`) :`NewEnumerator6` (`self.EQCommand`) :`NewEnumerator7` (`self.ResolutionCommand`) :`NewEnumerator8` (`self.ScreenCommand`) :`NewEnumerator9` (`self.MBCommand`) :`NewEnumerator10` (`self.VSyncCommand`) :`NewEnumerator11` (`self.ShadingCommand`)) StringType :!label _label))
    (:`NewEnumerator1`
      (goto _label))
    (:`NewEnumerator2`
      (goto _label))
    (:`NewEnumerator3`
      (goto _label))
    (:`NewEnumerator4`
      (goto _label))
    (:`NewEnumerator5`
      (goto _label))
    (:`NewEnumerator6`
      (goto _label))
    (:`NewEnumerator7`
      (goto _label))
    (:`NewEnumerator8`
      (goto _label))
    (:`NewEnumerator9`
      (goto _label))
    (:`NewEnumerator10`
      (goto _label))
    (:`NewEnumerator11`
      (goto _label))
    (:`NewEnumerator12`
      (`|VariableSetRef` (select `/Game/Blueprints/Enum_Settings` Type :`NewEnumerator12` (`self.MasterSound`) :`NewEnumerator13` (`self.Sensivity`)) FloatType :!label _label_2))
    (:`NewEnumerator13`
      (goto _label_2))
    (:`NewEnumerator14`
      (`|VariableSetRef` (select `/Game/Blueprints/Enum_Settings` Type :`NewEnumerator14` (`self.MouseInvert`)) BoolType)))
  (`GameplayStatics.SaveGameToSlot` self "Settings"))